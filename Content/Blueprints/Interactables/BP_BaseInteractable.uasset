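; Base interactable actor that shows a widget while the first-person player stands inside its sphere and opens a readable UI when interacted with.
; BeginPlay caches the player character, and sphere overlaps toggle the widget's visibility for that character only.
; Interaction plays a sound at the actor, then calls OnInteract, which creates the WidgetRef widget and adds it to the viewport.
; Leaving the sphere also removes that readable widget.
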(event OnComponentBeginOverlap(Sphere)
  (params (OverlappedComponent :type Primitive%20Component%20Object%20Reference) (OtherActor :type Actor%20Object%20Reference) (OtherComp :type Primitive%20Component%20Object%20Reference) (OtherBodyIndex :type Integer) (bFromSweep :type Boolean) (SweepResult :type Hit%20Result%20Structure%20%28by%20ref%29))
  (if (== OtherActor (Variables|Default|GetPlayerCharacter))
    (Rendering|SetVisibility (Variables|Default|GetWidget) true false)))

(event OnComponentEndOverlap(Sphere)
  (params (OverlappedComponent :type Primitive%20Component%20Object%20Reference) (OtherActor :type Actor%20Object%20Reference) (OtherComp :type Primitive%20Component%20Object%20Reference) (OtherBodyIndex :type Integer))
  (if (== OtherActor (Variables|Default|GetPlayerCharacter))
    (Rendering|SetVisibility (Variables|Default|GetWidget) false false)
    (Widget|RemovefromParent (Variables|Default|GetReadableWidget))))

(event Custom|OnInteract
  (bind _returnvalue (UserInterface|CreateWidget (Variables|Default|GetWidgetRef) (Game|GetPlayerController 0)))
  (bind _output_get (Variables|Default|SetReadableWidget _returnvalue))
  (UserInterface|Viewport|AddtoViewport _output_get 0))

(event EventBeginPlay
  (bind _asbp_first_person_character (Utilities|Casting|CastToBP_FirstPersonCharacter (Game|GetPlayerCharacter 0)))
  (Variables|Default|SetPlayerCharacter _asbp_first_person_character))

(event EventInteraction
  (Audio|PlaySoundatLocation (Variables|Default|GetSound) (Transformation|GetActorLocation) "0, 0, 0" 1.0 1.0 0.0 0 0 0 0)
  (CallFunction|OnInteract))

(fn ConstructionScript)